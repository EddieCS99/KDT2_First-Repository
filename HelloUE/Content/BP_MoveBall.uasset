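; BP_MoveBall is an actor that shuttles its static mesh back and forth along relative X between two fixed bounds.
; Each Tick moves the mesh by Speed scaled by delta time, and the MoveLever boolean flips direction at each bound.
; The mesh also rotates on the outbound leg only, by a fixed per-frame step that makes the spin frame-rate dependent.
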(event EventTick
  (params (DeltaSeconds :type Float%20%28single-precision%29))
  (bind _staticmesh (Variables|Default|GetStaticMesh))
  (bind _staticmesh_2 (Variables|Default|GetStaticMesh))
  (bind _speed (Variables|Default|GetSpeed))
  (bind _returnvalue (* DeltaSeconds _speed))
  (if (Variables|Default|GetMoveLever)
    (Transformation|AddRelativeLocation _staticmesh_2 (Math|Vector|MakeVector _returnvalue 0.0 0.0) false false)
    (Transformation|AddRelativeRotation _staticmesh_2 "0.000000,5.000000,10.000000" false false)
    (if (>= (.x (Variables|/Script/Engine.SceneComponent|GetRelativeLocation _staticmesh_2)) 1e+03)
      (Variables|Default|SetMoveLever false))
    (else
      (Transformation|AddRelativeLocation _staticmesh (Math|Vector|MakeVector (* _returnvalue -1.0) 0.0 0.0) false false)
      (if (<= (.x (Variables|/Script/Engine.SceneComponent|GetRelativeLocation _staticmesh)) 0.0)
        (Variables|Default|SetMoveLever true)))))

(fn ConstructionScript)