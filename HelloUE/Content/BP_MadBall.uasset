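; BP_MadBall is a Blueprint that moves its MadBall component endlessly around a square loop in the relative XZ plane while tumbling it.
; Tick switches on MoveType, advancing the ball at Speed scaled by delta time and changing to the next state when it passes that side's limit.
; Each state also adds a fixed rotation per frame, so the spin, unlike the movement, depends on frame rate.
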(event EventTick
  (params (DeltaSeconds :type Float%20%28single-precision%29))
  (bind _speed (Variables|Default|GetSpeed))
  (bind _madball (Variables|Default|GetMadBall))
  (bind _madball_2 (Variables|Default|GetMadBall))
  (bind _madball_3 (Variables|Default|GetMadBall))
  (bind _madball_4 (Variables|Default|GetMadBall))
  (bind _returnvalue (* DeltaSeconds _speed))
  (switch Utilities|FlowControl|Switch|SwitchonEN_MadBall (Variables|Default|GetMoveType)
    (:NewEnumerator0
      (Transformation|AddRelativeLocation _madball (Math|Vector|MakeVector _returnvalue 0.0 0.0) false false)
      (Transformation|AddRelativeRotation _madball "0.000000,3.000000,7.000000" false false)
      (if (>= (.x (Variables|/Script/Engine.SceneComponent|GetRelativeLocation _madball)) 5e+02)
        (Variables|Default|SetMoveType "NewEnumerator1")))
    (:NewEnumerator1
      (Transformation|AddRelativeLocation _madball_2 (Math|Vector|MakeVector 0.0 0.0 _returnvalue) false false)
      (Transformation|AddRelativeRotation _madball_2 "0.000000,7.000000,3.000000" false false)
      (if (>= (.z (Variables|/Script/Engine.SceneComponent|GetRelativeLocation _madball_2)) 5e+02)
        (Variables|Default|SetMoveType "NewEnumerator2")))
    (:NewEnumerator2
      (Transformation|AddRelativeLocation _madball_3 (Math|Vector|MakeVector (* _returnvalue -1.0) 0.0 0.0) false false)
      (Transformation|AddRelativeRotation _madball_3 "0.000000,3.000000,7.000000" false false)
      (if (<= (.x (Variables|/Script/Engine.SceneComponent|GetRelativeLocation _madball_3)) 0.0)
        (Variables|Default|SetMoveType "NewEnumerator3")))
    (:NewEnumerator3
      (Transformation|AddRelativeLocation _madball_4 (Math|Vector|MakeVector 0.0 0.0 (* _returnvalue -1.0)) false false)
      (Transformation|AddRelativeRotation _madball_4 "0.000000,7.000000,3.000000" false false)
      (if (<= (.z (Variables|/Script/Engine.SceneComponent|GetRelativeLocation _madball_4)) 0.0)
        (Variables|Default|SetMoveType "NewEnumerator0")))))

(fn ConstructionScript)