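; BP_MoveLeftRight is an actor whose Sphere component shuttles back and forth along its relative X axis while tumbling.
; Each Tick, a MoveLever boolean picks the direction, flipping at positive and negative X limits, with faster forward travel and a different spin each way.
; Movement is a fixed per-frame step without delta time, so speed depends on frame rate.
; Disconnected practice snippets for printing, loops and time counting never run.
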(event EventBeginPlay
  ;[1 1 1 1 25] 이벤트
)

(event EventTick
  (params (DeltaSeconds :type Float%20%28single-precision%29))
  (bind _sphere (Variables|Default|GetSphere))
  (bind _sphere_2 (Variables|Default|GetSphere))
  ;[0 1 0.8801 1 20] 00축으로 이동 후 반복
  (if (Variables|Default|GetMoveLever)
    (Transformation|AddRelativeLocation _sphere_2 "15.000000,0.000000,0.000000" false false)
    (Transformation|AddLocalRotation _sphere_2 "0.000000,10.000000,5.000000" false false)
    (if (>= (.x (Variables|/Script/Engine.SceneComponent|GetRelativeLocation _sphere_2)) 1e+03)
      (Variables|Default|SetMoveLever false))
    (else
      (Transformation|AddRelativeLocation _sphere "-5.000000,0.000000,0.000000" false false)
      (Transformation|AddLocalRotation _sphere "0.000000,5.000000,10.000000" false false)
      (if (<= (.x (Variables|/Script/Engine.SceneComponent|GetRelativeLocation _sphere)) -1e+03)
        (Variables|Default|SetMoveLever true)))))

(fn ConstructionScript)